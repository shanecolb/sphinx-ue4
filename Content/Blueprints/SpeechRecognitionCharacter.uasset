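; Character Blueprint that demonstrates keyword speech recognition through a spawned SpeechRecognitionActor.
; BeginPlay spawns the actor and binds its OnWordSpoken event to a handler that prints the recognized text.
; The I key initializes English recognition with a short list of keyword phrases and prints success or failure.
; The S key and EndPlay shut the recognizer down.
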(event Custom|Event%20Word%20Spoken
  (params (Text :type String))
  ;[1 1 1] Create Speech Recognition Actor, and sets up word spoken event
  (CallFunction|WordSpoken Text))

(event EventBeginPlay
  ;[1 1 1] Create Speech Recognition Actor, and sets up word spoken event
  (bind _returnvalue (Game|SpawnActorfromClass "/Script/SpeechRecognition.SpeechRecognitionActor" (Transformation|GetActorTransform) "Undefined" 0 0))
  (bind _output_get (Variables|Default|SetSpeechRecognition_ptr _returnvalue))
  (EventDispatchers|AssignOnWordSpoken _output_get (delegate Custom|Event%20Word%20Spoken)))

(event EventActorBeginOverlap
  (params (OtherActor :type Actor%20Object%20Reference))
  ;[1 1 1] Create Speech Recognition Actor, and sets up word spoken event
)

(event EventTick
  (params (DeltaSeconds :type Float%20%28single-precision%29)))

(event EventEndPlay
  (params (EndPlayReason :type EEndPlayReason%20Enum :default "Destroyed"))
  (Class|SpeechRecognitionActor|Shutdown (Variables|Default|GetSpeechRecognition_ptr)))

(event Input|KeyboardEvents|I
  (params (Key :type Key%20Structure :default "AnyKey"))
  (:Pressed
    (bind _returnvalue (Class|SpeechRecognitionActor|Init (Variables|Default|GetSpeechRecognition_ptr) "VE_English" (Utilities|Array|MakeArray (Utilities|Struct|MakeRecognitionPhrase "close browser" "VE_5") (Utilities|Struct|MakeRecognitionPhrase "open browser" "VE_5") (Utilities|Struct|MakeRecognitionPhrase "hello world" "VE_5"))))
    (if _returnvalue
      (Development|PrintString "Speech Recognition Init : SUCCESS")
      (else
        (Development|PrintString "Speech Recognition Init : FAILURE")))))

(event Input|KeyboardEvents|S
  (params (Key :type Key%20Structure :default "AnyKey"))
  (:Pressed
    (Class|SpeechRecognitionActor|Shutdown (Variables|Default|GetSpeechRecognition_ptr))))

(fn ConstructionScript)

(fn WordSpoken
  (params (FString :type String))
  (Development|PrintString FString))